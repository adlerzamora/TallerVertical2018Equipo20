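; Traffic light actor (semaforo) that loops through green, yellow and red phases, holding yellow for less time than the others.
; A single Light component teleports between three component positions stored in an array and takes the color matching the current index.
; Tick drives the cycle: it refreshes light and color, while a phase-length Delay gates each index step.
; A separate RedLight component is visible only during red.
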(event `self.ReceiveBeginPlay`
  (set `self.Pos` (`|MakeArray` (`self.Pos0`) (`self.StaticMesh1`) (`self.StaticMesh2`))))

(event `self.ReceiveTick`
  (params (DeltaSeconds :type "Float (single-precision)"))
  (bind _pos_index (`self.Pos_INDEX`))
  (bind _red_light (`self.Red_light`))
  (`|ExecutionSequence`
    (:`then_0`
      (if (== (`self.Pos_INDEX`) 2)
        (`SceneComponent.SetVisibility` _red_light true false)
        (`self.Set_LocAndColor`)
        (else
          (`SceneComponent.SetVisibility` _red_light false false)
          (`self.Set_LocAndColor`)))
      (`self.Time`)
      (`KismetSystemLibrary.Delay` (`self.Time_`))
      (if (== (- (`KismetArrayLibrary.Array_Length` (`self.Pos`)) 1) _pos_index)
        (set `self.Pos_INDEX` 0)
        (else
          (`/Engine/EditorBlueprintResources/StandardMacros.IncrementInt` _pos_index))))
    (:`then_1`
      (`self.Switch_Color`))))

(fn `Set_LocAndColor`
  (bind _light (`self.Light`))
  (`SceneComponent.K2_SetRelativeLocation` _light (`SceneComponent.RelativeLocation` (`|GetArrayItem` (`self.Pos`) (`self.Pos_INDEX`))) false true)
  (`LightComponent.SetLightColor` _light (`self.Color`) true))

(fn `Switch_Color`
  (switch `int` (`self.Pos_INDEX`)
    (:`0`
      (set `self.Color` (struct :`R` 0.062751 :`G` 0.382365 :`A` 1.0)))
    (:`1`
      (set `self.Color` (struct :`R` 0.382365 :`G` 0.348352 :`A` 1.0)))
    (:`2`
      (set `self.Color` (struct :`R` 0.382365 :`B` 0.01097 :`A` 1.0)))))

(fn `Time`
  (switch `int` (`self.Pos_INDEX`)
    (:`0`
      (set `self.Time_` 5.0))
    (:`1`
      (set `self.Time_` 2.0))
    (:`2`
      (set `self.Time_` 5.0))))

(fn `UserConstructionScript`)