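; Cartera (wallet) actor that can be picked up and dropped, and plays a heartbeat cue paced by its distance to the player.
; Two custom events attach it to a given component with physics off, or detach it with physics back on.
; A looping timer, its period fixed from the BeginPlay distance, repeatedly resets the heartbeat timer to a clamped distance-based interval, shorter when the player is nearer.
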(event `CustomEvent`
  (params (AttachTo :type "SceneComponent Object Reference"))
  (`PrimitiveComponent.SetSimulatePhysics` (`self.StaticMeshComponent`) false)
  (`SceneComponent.K2_AttachToComponent` (`self.K2_GetRootComponent`) AttachTo "None" "KeepWorld" "KeepWorld" "KeepWorld" false))

(event `CustomEvent_1`
  (`PrimitiveComponent.SetSimulatePhysics` (`self.StaticMeshComponent`) true)
  (`self.K2_DetachFromActor` "KeepWorld" "KeepWorld" "KeepWorld"))

(event `self.ReceiveBeginPlay`
  (`KismetSystemLibrary.K2_SetTimerDelegate` (delegate `Update Time`) (`KismetMathLibrary.FClamp` (/ (`self.GetDistanceTo` (`GameplayStatics.GetPlayerPawn` 0)) 800.0) 0.81 5.0) true))

(event `Update Time`
  (`KismetSystemLibrary.K2_SetTimerDelegate` (delegate `Play Heart`) (- (`KismetMathLibrary.FClamp` (/ (`self.GetDistanceTo` (`GameplayStatics.GetPlayerPawn` 0)) 800.0) 0.81 5.0) 0.005) true))

(event `Play Heart`
  (`AudioComponent.Play` (`self.Singlebeat_Cue`) 0.0))

(fn `UserConstructionScript`)